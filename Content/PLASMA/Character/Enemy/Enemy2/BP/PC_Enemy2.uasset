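; AI controller for Enemy2 that caches the possessed CH_Enemy2 pawn and starts the BT_Enemy2 behavior tree.
; AI perception updates on the main character set the CanSeePlayer blackboard flag, and losing sight also stores the player's current location and sets RecentlySighted.
; Walk, Run and attack events forward to the matching functions on the pawn.
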(event OnTargetPerceptionUpdated(AIPerception)
  (params (Actor :type Actor%20Object%20Reference) (Stimulus :type AI%20Stimulus%20Structure))
  (bind _bsuccessfullysensed (Utilities|Struct|BreakAIStimulus Stimulus))
  (bind _returnvalue (AI|GetBlackboard 0))
  (Utilities|Casting|CastToCH_Main Actor)
  (AI|Components|Blackboard|SetValueasBool _returnvalue (Utilities|Name|MakeLiteralName "CanSeePlayer") _bsuccessfullysensed)
  (if (not _bsuccessfullysensed)
    (AI|Components|Blackboard|SetValueasVector _returnvalue (Utilities|Name|MakeLiteralName "PlayerLocation") (Transformation|GetActorLocation (Game|GetPlayerCharacter 0)))
    (AI|Components|Blackboard|SetValueasBool _returnvalue (Utilities|Name|MakeLiteralName "RecentlySighted") true)))

(event Custom|Walk
  (Default|Walk (Variables|Default|GetRef_Enemy2)))

(event Custom|attack
  (Default|Attack (Variables|Default|GetRef_Enemy2)))

(event Custom|Run
  (Default|Run (Variables|Default|GetRef_Enemy2)))

(event EventOnPossess
  (params (PossessedPawn :type Pawn%20Object%20Reference))
  (bind _asch_enemy_2 (Utilities|Casting|CastToCH_Enemy2 PossessedPawn))
  (Variables|Default|SetRef_Enemy2 _asch_enemy_2)
  (AI|RunBehaviorTree "/Game/PLASMA/Character/Enemy/Enemy2/BP/BT_Enemy2.BT_Enemy2"))

(fn ConstructionScript)